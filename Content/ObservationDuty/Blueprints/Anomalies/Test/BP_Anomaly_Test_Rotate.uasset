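; Test anomaly actor for Observation Duty that spins around its yaw axis while its anomaly is active.
; Tick checks the Anomaly member's active state and adds RotationSpeed scaled by delta time to the actor's yaw.
; The activation event caches the starting rotation, and deactivation restores it.
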(event OnAnomalyActivatedEvent(Anomaly)
  (Variables|Default|SetCachedRotation (Transformation|GetActorRotation)))

(event OnAnomalyDeactivatedEvent(Anomaly)
  (Transformation|SetActorRotation (Variables|Default|GetCachedRotation)))

(event EventTick
  (params (DeltaSeconds :type Float%20%28single-precision%29))
  (bind _returnvalue (Transformation|GetActorRotation))
  (if (Class|AnomalyComponent|IsAnomalyActive (Variables|Default|GetAnomaly))
    (Transformation|SetActorRotation (Math|Rotator|MakeRotator (.roll _returnvalue) (.pitch _returnvalue) (+ (.yaw _returnvalue) (* (Variables|Default|GetRotationSpeed) DeltaSeconds))))))

(fn ConstructionScript)