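; BP_Anomaly_Test_Scale is a test anomaly for Observation Duty that continuously changes its actor's scale while the anomaly is active.
; On activation, it caches the current scale and resets the multiplier to one.
; Tick advances the multiplier by ScaleSpeed over time and applies it to the cached scale.
; Deactivation restores the cached scale.
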(event OnAnomalyActivatedEvent(Anomaly)
  (Variables|Default|SetCachedScale (Transformation|GetActorScale3D))
  (Variables|Default|SetScaleMultiplier 1.0))

(event OnAnomalyDeactivatedEvent(Anomaly)
  (Transformation|SetActorScale3D (Variables|Default|GetCachedScale)))

(event EventTick
  (params (DeltaSeconds :type Float%20%28single-precision%29))
  (if (Class|AnomalyComponent|IsAnomalyActive (Variables|Default|GetAnomaly))
    (bind _output_get (Variables|Default|SetScaleMultiplier (+ (Variables|Default|GetScaleMultiplier) (* (Variables|Default|GetScaleSpeed) DeltaSeconds))))
    (Transformation|SetActorScale3D (* _output_get (Variables|Default|GetCachedScale)))))

(fn ConstructionScript)